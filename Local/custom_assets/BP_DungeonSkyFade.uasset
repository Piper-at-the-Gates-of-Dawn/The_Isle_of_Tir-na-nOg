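; BP_DungeonSkyFade is a box trigger that swaps a DynamicSkyNormal area's settings between dungeon and default values.
; On BeginPlay it finds the AreaSpecificSettings index whose name matches AreaToHijack, or disables box collision on dedicated servers.
; Any begin or end overlap calls MoveArea, which hijacks that existing area by rewriting its center, volume, priority, radius and fade exponent.
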(event `self.ReceiveBeginPlay`
  (if (`KismetSystemLibrary.IsDedicatedServer`)
    (`PrimitiveComponent.SetCollisionEnabled` (`self.Box`) "NoCollision")
    (else
      (for (_array_element _array_index) (`/Game/Marketplace/UltraDynamicSky/Blueprints/Ultra_Dynamic_Sky_BP.AreaSpecificSettings` (`self.DynamicSky_Normal`))
        (if (== (`.name_51_01DB10B1486BB2EFEDBD38905F20E0DF` (break `/Game/Marketplace/UltraDynamicSky/Blueprints/SkyCurveSet` _array_element)) (`self.AreaToHijack`))
          (set `self.AreaSpecificSettingsIndex` _array_index)
          (break))))))

(event `self.Box.OnComponentBeginOverlap`
  (params (OverlappedComponent :type "PrimitiveComponent Object Reference") (OtherActor :type "Actor Object Reference") (OtherComp :type "PrimitiveComponent Object Reference") (OtherBodyIndex :type Integer) (bFromSweep :type Boolean) (SweepResult :type "HitResult Structure (by ref)"))
  (`KismetSystemLibrary.PrintString` "Entered")
  (`self.MoveArea` true))

(event `self.Box.OnComponentEndOverlap`
  (params (OverlappedComponent :type "PrimitiveComponent Object Reference") (OtherActor :type "Actor Object Reference") (OtherComp :type "PrimitiveComponent Object Reference") (OtherBodyIndex :type Integer))
  (`KismetSystemLibrary.PrintString` "Exited")
  (`self.MoveArea` false))

(fn `MoveArea`
  (params (Entered :type Boolean))
  (`/Game/Marketplace/UltraDynamicSky/Blueprints/Ultra_Dynamic_Sky_BP.SetAreaSpecificParams` (`self.DynamicSky_Normal`) (`self.AreaSpecificSettingsIndex`) (make `EnvironmentArea` (select `bool` Entered :`false` (`self.DefaultLocation`) :`true` (`self.DungeonLocation`)) (select `bool` Entered :`false` (`self.DefaultVolume`) :`true` (`self.DungeonVolume`)) (select `bool` Entered :`false` (`self.DefaultPriority`) :`true` (`self.DungeonPriority`)) (select `bool` Entered :`false` (`self.DefaultRadius`) :`true` (`self.DungeonRadius`)) (select `bool` Entered :`false` (`self.DefaultFadeExponent`) :`true` (`self.DungeonFadeExponent`)))))

(fn `UserConstructionScript`)